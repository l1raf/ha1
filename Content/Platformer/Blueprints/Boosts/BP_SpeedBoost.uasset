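; BP_SpeedBoost is a platformer pickup with a spinning crystal that, despite its name, triggers the game mode's slowdown.
; BeginPlay caches the ThirdPersonGameMode, and Tick rotates the crystal at RotationSpeed.
; When a ThirdPersonCharacter overlaps it and Bonuses cover SlowdownCost, it destroys every actor tagged "Boost" so only one boost is usable, then calls ActivateSlowdown.
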(event `self.ReceiveBeginPlay`
  (bind _asthird_person_game_mode (cast `/Game/ThirdPersonBP/Blueprints/ThirdPersonGameMode` (`GameplayStatics.GetGameMode`)))
  (set `self.GameMode` _asthird_person_game_mode))

(event `self.ReceiveActorBeginOverlap`
  (params (OtherActor :type "Actor Object Reference"))
  (bind _gamemode (`self.GameMode`))
  (cast `/Game/ThirdPersonBP/Blueprints/ThirdPersonCharacter` OtherActor)
  (if (>= (`/Game/ThirdPersonBP/Blueprints/ThirdPersonGameMode.Bonuses` _gamemode) (`/Game/ThirdPersonBP/Blueprints/ThirdPersonGameMode.SlowdownCost` _gamemode))
    ;[1 1 1] Only one boost can be used at a time, so destroy both when one is collected
    (bind _outactors (`GameplayStatics.GetAllActorsWithTag` "Boost"))
    (for _array_element _outactors
      (`self.K2_DestroyActor` _array_element))
    (`/Game/ThirdPersonBP/Blueprints/ThirdPersonGameMode.ActivateSlowdown` (`self.GameMode`))))

(event `self.ReceiveTick`
  (params (DeltaSeconds :type "Float (single-precision)"))
  (`SceneComponent.K2_AddLocalRotation` (`self.Crystal`) (* (`KismetMathLibrary.MakeRotator` 0.0 0.0 (`self.RotationSpeed`)) DeltaSeconds) false false))

(fn `UserConstructionScript`)