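; BP_Platform2 is a platformer platform variant with a wall obstacle on it, extending a parent platform Blueprint.
; On BeginPlay it rotates the Platform 90 degrees in yaw and randomizes the Wall's thickness and height through relative scale.
; While the game mode's WallsBoostActivated flag is set, the character's actor overlap disables Wall collision, and end overlap restores it, letting the player pass through.
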(event `self.ReceiveBeginPlay`
  (`parent.ReceiveBeginPlay`)
  (`SceneComponent.K2_AddLocalRotation` (`self.Platform`) (`KismetMathLibrary.MakeRotator` 0.0 0.0 90.0) false false)
  (`SceneComponent.SetRelativeScale3D` (`self.Wall`) (`KismetMathLibrary.MakeVector` 1.0 (`KismetMathLibrary.RandomFloatInRange` 0.1 0.2) (`KismetMathLibrary.RandomFloatInRange` 1.0 3.0))))

(event `self.ReceiveActorBeginOverlap`
  (params (OtherActor :type "Actor Object Reference"))
  (cast `/Game/ThirdPersonBP/Blueprints/ThirdPersonCharacter` OtherActor)
  (if (`/Game/ThirdPersonBP/Blueprints/ThirdPersonGameMode.WallsBoostActivated` (`self.GameMode`))
    (`PrimitiveComponent.SetCollisionEnabled` (`self.Wall`) "NoCollision")))

(event `self.ReceiveActorEndOverlap`
  (params (OtherActor :type "Actor Object Reference"))
  (cast `/Game/ThirdPersonBP/Blueprints/ThirdPersonCharacter` OtherActor)
  (if (`/Game/ThirdPersonBP/Blueprints/ThirdPersonGameMode.WallsBoostActivated` (`self.GameMode`))
    (`PrimitiveComponent.SetCollisionEnabled` (`self.Wall`) "QueryAndPhysics")))

(fn `UserConstructionScript`
  (`parent.UserConstructionScript`))