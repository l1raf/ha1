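; Spike hazard platform for the platformer that kills the player on contact by destroying any overlapping ThirdPersonCharacter.
; It extends a parent Blueprint, running that BeginPlay first, then giving the Platform component a 90-degree yaw half the time when Movable is set.
; Tick is disabled and the construction script only calls the parent.
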(event `self.ReceiveBeginPlay`
  (`parent.ReceiveBeginPlay`)
  (if (and (`self.Movable`) (< (`KismetMathLibrary.RandomFloat`) 0.5))
    (`SceneComponent.K2_AddLocalRotation` (`self.Platform`) (`KismetMathLibrary.MakeRotator` 0.0 0.0 90.0) false false)))

(event `self.ReceiveActorBeginOverlap`
  (params (OtherActor :type "Actor Object Reference"))
  (bind _asthird_person_character (cast `/Game/ThirdPersonBP/Blueprints/ThirdPersonCharacter` OtherActor))
  (`self.K2_DestroyActor` _asthird_person_character))

(fn `UserConstructionScript`
  (`parent.UserConstructionScript`))