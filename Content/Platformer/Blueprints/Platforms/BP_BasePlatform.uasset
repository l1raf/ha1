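; Base platform Blueprint for a platformer that randomly spawns a coin when play begins.
; On BeginPlay, an 80% random roll gates a single SpawnActor call owned by the platform.
; The spawn X is randomly offset from the root component's world location, while Y and Z are random absolute world values, independent of the platform's position.
; The construction script is empty.
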(event `self.ReceiveBeginPlay`
  (bind _returnvalue_x (`KismetMathLibrary.BreakVector` (`SceneComponent.K2_GetComponentLocation` (`self.DefaultSceneRoot`))))
  ;[1 1 1] Spawn coin with 80% probability
  (if (< (`KismetMathLibrary.RandomFloat`) 0.8)
    (`|SpawnActorFromClass` "/Game/Platformer/Blueprints/BP_Bonus.BP_Bonus_C" (`KismetMathLibrary.MakeTransform` (`KismetMathLibrary.MakeVector` (+ _returnvalue_x (`KismetMathLibrary.RandomFloatInRange` -400.0 400.0)) (`KismetMathLibrary.RandomFloatInRange` -400.0 400.0) (`KismetMathLibrary.RandomFloatInRange` 100.0 200.0))) "Undefined" "OverrideRootScale" self null)))

(fn `UserConstructionScript`)