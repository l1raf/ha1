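; Falling platform for a platformer level that sinks while the third-person character overlaps it and moves back along the same path when they leave.
; The FallMove timeline drives the platform mesh's relative Z, playing on overlap begin and reversing on overlap end.
; Its play rate scales with the game mode's Level, and each update lowers it to a clamped minimum while the slowdown boost is active.
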(event `self.ReceiveBeginPlay`
  (`parent.ReceiveBeginPlay`)
  (bind _asthird_person_game_mode (cast `/Game/ThirdPersonBP/Blueprints/ThirdPersonGameMode` (`GameplayStatics.GetGameMode`)))
  (bind _output_get (set `self.GameMode` _asthird_person_game_mode))
  (bind _output_get_2 (set `self.FallSpeed` (/ (`KismetMathLibrary.Conv_IntToDouble` (`/Game/ThirdPersonBP/Blueprints/ThirdPersonGameMode.Level` _output_get)) 5.0)))
  (`TimelineComponent.SetPlayRate` (`self.FallMove`) _output_get_2))

(event `self.ReceiveActorBeginOverlap`
  (params (OtherActor :type "Actor Object Reference"))
  (cast `/Game/ThirdPersonBP/Blueprints/ThirdPersonCharacter` OtherActor)
  (bind (_direction _newtrack_0) (`Timeline|FallMove` :!label _label)
    (:`Update`
      (`SceneComponent.K2_SetRelativeLocation` (`self.Platform`) (`KismetMathLibrary.MakeVector` 0.0 0.0 _newtrack_0) false false)
      ;[1 1 1] Change fall speed if slowdown boost is activated
      (if (`/Game/ThirdPersonBP/Blueprints/ThirdPersonGameMode.SlowdownActivated` (`self.GameMode`))
        (`TimelineComponent.SetPlayRate` (`self.FallMove`) (`KismetMathLibrary.FMax` (- (`self.FallSpeed`) (`/Game/ThirdPersonBP/Blueprints/ThirdPersonGameMode.SlowDownValue` (`self.GameMode`))) 0.2))
        (else
          (`TimelineComponent.SetPlayRate` (`self.FallMove`) (`self.FallSpeed`)))))))

(event `self.ReceiveActorEndOverlap`
  (params (OtherActor :type "Actor Object Reference"))
  (cast `/Game/ThirdPersonBP/Blueprints/ThirdPersonCharacter` OtherActor)
  (goto _label :!via `Reverse`))

(fn `UserConstructionScript`)