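; BP_KnockingOffPlatform is a platform whose wall slides sideways to knock the player off when the character steps on it.
; Overlap by the ThirdPersonCharacter plays the MoveWall timeline that drives the wall's relative Y location, and leaving reverses it.
; Timeline speed scales with the game mode's Level and drops, with a floor, during slowdown boost.
; An active walls boost disables wall collision during overlap.
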(event `self.ReceiveBeginPlay`
  (`parent.ReceiveBeginPlay`)
  (bind _asthird_person_game_mode (cast `/Game/ThirdPersonBP/Blueprints/ThirdPersonGameMode` (`GameplayStatics.GetGameMode`)))
  (bind _output_get (set `self.GameMode` _asthird_person_game_mode))
  (bind _output_get_2 (set `self.Speed` (/ (`KismetMathLibrary.Conv_IntToDouble` (`/Game/ThirdPersonBP/Blueprints/ThirdPersonGameMode.Level` _output_get)) 2.0)))
  (`TimelineComponent.SetPlayRate` (`self.MoveWall`) _output_get_2))

(event `self.ReceiveActorBeginOverlap`
  (params (OtherActor :type "Actor Object Reference"))
  (cast `/Game/ThirdPersonBP/Blueprints/ThirdPersonCharacter` OtherActor)
  (if (`/Game/ThirdPersonBP/Blueprints/ThirdPersonGameMode.WallsBoostActivated` (`self.GameMode`))
    (`PrimitiveComponent.SetCollisionEnabled` (`self.Wall`) "NoCollision")
    (bind (_direction _newtrack_0) (`Timeline|MoveWall` :!label _label)
      (:`Update`
        (`SceneComponent.K2_SetRelativeLocation` (`self.Wall`) (`KismetMathLibrary.MakeVector` 0.0 _newtrack_0 100.0) false false)
        ;[1 1 1] Change move speed if slowdown boost is activated
        (if (`/Game/ThirdPersonBP/Blueprints/ThirdPersonGameMode.SlowdownActivated` (`self.GameMode`))
          (`TimelineComponent.SetPlayRate` (`self.MoveWall`) (`KismetMathLibrary.FMax` (- (`self.Speed`) (`/Game/ThirdPersonBP/Blueprints/ThirdPersonGameMode.SlowDownValue` (`self.GameMode`))) 0.5))
          (else
            (`TimelineComponent.SetPlayRate` (`self.MoveWall`) (`self.Speed`))))))
    (else
      (goto _label))))

(event `self.ReceiveActorEndOverlap`
  (params (OtherActor :type "Actor Object Reference"))
  (cast `/Game/ThirdPersonBP/Blueprints/ThirdPersonCharacter` OtherActor)
  (if (`/Game/ThirdPersonBP/Blueprints/ThirdPersonGameMode.WallsBoostActivated` (`self.GameMode`))
    (`PrimitiveComponent.SetCollisionEnabled` (`self.Wall`) "QueryAndPhysics")
    (goto _label :!via `Reverse`)
    (else
      (goto _label :!via `Reverse`))))

(fn `UserConstructionScript`)