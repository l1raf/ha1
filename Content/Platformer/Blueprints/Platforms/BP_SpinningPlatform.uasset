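; Platformer platform actor that spins continuously around its yaw axis.
; On BeginPlay it reads the Level from the ThirdPersonGameMode and scales its rotation speed with it, so higher levels spin faster.
; Tick applies a frame-rate independent local yaw rotation to the Platform component.
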(event `self.ReceiveBeginPlay`
  (bind _asthird_person_game_mode (cast `/Game/ThirdPersonBP/Blueprints/ThirdPersonGameMode` (`GameplayStatics.GetGameMode`)))
  (bind _output_get (set `self.GameMode` _asthird_person_game_mode))
  (set `self.RotationSpeed` (* (`/Game/ThirdPersonBP/Blueprints/ThirdPersonGameMode.Level` _output_get) 5.0)))

(event `self.ReceiveTick`
  (params (DeltaSeconds :type "Float (single-precision)"))
  (`SceneComponent.K2_AddLocalRotation` (`self.Platform`) (* (`KismetMathLibrary.MakeRotator` 0.0 0.0 (`self.RotationSpeed`)) DeltaSeconds) false false))

(fn `UserConstructionScript`)