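; Spinning wall platform for a platformer level, with a wall that yaws continuously at a speed scaled by the game mode's current Level.
; Tick rotates the Wall component, reducing its speed down to a fixed minimum while the game mode's slowdown is active.
; While the walls boost is active, the Wall's collision is disabled when the player character begins overlapping the actor and restored when the overlap ends.
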(event `self.ReceiveBeginPlay`
  (`parent.ReceiveBeginPlay`)
  (bind _asthird_person_game_mode (cast `/Game/ThirdPersonBP/Blueprints/ThirdPersonGameMode` (`GameplayStatics.GetGameMode`)))
  (bind _output_get (set `self.GameMode` _asthird_person_game_mode))
  (set `self.RotationSpeed` (* (`/Game/ThirdPersonBP/Blueprints/ThirdPersonGameMode.Level` _output_get) 10.0)))

(event `self.ReceiveTick`
  (params (DeltaSeconds :type "Float (single-precision)"))
  (if (`/Game/ThirdPersonBP/Blueprints/ThirdPersonGameMode.SlowdownActivated` (`self.GameMode`))
    (`SceneComponent.K2_AddLocalRotation` (`self.Wall`) (* (`KismetMathLibrary.MakeRotator` 0.0 0.0 (`KismetMathLibrary.FMax` (- (`self.RotationSpeed`) (* 10 (`/Game/ThirdPersonBP/Blueprints/ThirdPersonGameMode.SlowDownValue` (`self.GameMode`)))) 10.0)) DeltaSeconds) false false)
    (else
      (`SceneComponent.K2_AddLocalRotation` (`self.Wall`) (* (`KismetMathLibrary.MakeRotator` 0.0 0.0 (`self.RotationSpeed`)) DeltaSeconds) false false))))

(event `self.ReceiveActorBeginOverlap`
  (params (OtherActor :type "Actor Object Reference"))
  (cast `/Game/ThirdPersonBP/Blueprints/ThirdPersonCharacter` OtherActor)
  (if (`/Game/ThirdPersonBP/Blueprints/ThirdPersonGameMode.WallsBoostActivated` (`self.GameMode`))
    (`PrimitiveComponent.SetCollisionEnabled` (`self.Wall`) "NoCollision")))

(event `self.ReceiveActorEndOverlap`
  (params (OtherActor :type "Actor Object Reference"))
  (cast `/Game/ThirdPersonBP/Blueprints/ThirdPersonCharacter` OtherActor)
  (if (`/Game/ThirdPersonBP/Blueprints/ThirdPersonGameMode.WallsBoostActivated` (`self.GameMode`))
    (`PrimitiveComponent.SetCollisionEnabled` (`self.Wall`) "QueryAndPhysics")))

(fn `UserConstructionScript`)