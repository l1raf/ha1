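; Platformer platform that, if flagged Movable, has a 50% chance on BeginPlay to move.
; A second coin flip picks the Movement timeline for relative Y motion or Timeline_0 for relative Z motion.
; Play rate derives from the game mode's Level, reduced while slowdown is active but clamped to a minimum.
; Both branches set that rate only on Movement, so vertical motion ignores level and slowdown.
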(event `self.ReceiveBeginPlay`
  ;[1 1 1] Make platform moving with 50% probability
  (bind _asthird_person_game_mode (cast `/Game/ThirdPersonBP/Blueprints/ThirdPersonGameMode` (`GameplayStatics.GetGameMode`)))
  (set `self.GameMode` _asthird_person_game_mode)
  (if (and (`self.Movable`) (< (`KismetMathLibrary.RandomFloat`) 0.5))
    (`self.InitVars`)
    (if (< (`KismetMathLibrary.RandomFloat`) 0.5)
      (bind (_direction _newtrack_0) (`Timeline|Movement`)
        (:`Update`
          (`SceneComponent.K2_SetRelativeLocation` (`self.Platform`) (`KismetMathLibrary.MakeVector` 0.0 _newtrack_0) false false)))
      (else
        (bind (_direction_2 _newtrack_0_2) (`Timeline|Timeline_0`)
          (:`Update`
            (`SceneComponent.K2_SetRelativeLocation` (`self.Platform`) (`KismetMathLibrary.MakeVector` 0.0 0.0 _newtrack_0_2) false false)))))
    ;[1 1 1] Change move speed if slowdown boost is activated
    (if (`/Game/ThirdPersonBP/Blueprints/ThirdPersonGameMode.SlowdownActivated` (`self.GameMode`))
      (`TimelineComponent.SetPlayRate` (`self.Movement`) (`KismetMathLibrary.FMax` (- (`self.Duration`) (`/Game/ThirdPersonBP/Blueprints/ThirdPersonGameMode.SlowDownValue` (`self.GameMode`))) 1.0))
      (else
        (`TimelineComponent.SetPlayRate` (`self.Movement`) (`self.Duration`))))))

(fn `InitVars`
  (bind _output_get (set `self.Duration` (`KismetMathLibrary.Conv_IntToDouble` (`/Game/ThirdPersonBP/Blueprints/ThirdPersonGameMode.Level` (`self.GameMode`)))))
  (`TimelineComponent.SetPlayRate` (`self.Movement`) _output_get))

(fn `UserConstructionScript`)