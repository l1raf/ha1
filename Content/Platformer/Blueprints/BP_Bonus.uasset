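; BP_Bonus is a collectible coin pickup for the platformer.
; It caches the ThirdPersonGameMode on BeginPlay and spins its Coin component around yaw every tick at RotationSpeed.
; When a ThirdPersonCharacter overlaps it, the actor destroys itself and calls BonusCollected on the game mode.
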(event `self.ReceiveBeginPlay`
  (bind _asthird_person_game_mode (cast `/Game/ThirdPersonBP/Blueprints/ThirdPersonGameMode` (`GameplayStatics.GetGameMode`)))
  (set `self.GameMode` _asthird_person_game_mode))

(event `self.ReceiveActorBeginOverlap`
  (params (OtherActor :type "Actor Object Reference"))
  (cast `/Game/ThirdPersonBP/Blueprints/ThirdPersonCharacter` OtherActor)
  (`self.K2_DestroyActor`)
  (`/Game/ThirdPersonBP/Blueprints/ThirdPersonGameMode.BonusCollected` (`self.GameMode`)))

(event `self.ReceiveTick`
  (params (DeltaSeconds :type "Float (single-precision)"))
  (`SceneComponent.K2_AddLocalRotation` (`self.Coin`) (* (`KismetMathLibrary.MakeRotator` 0.0 0.0 (`self.RotationSpeed`)) DeltaSeconds) false false))

(fn `UserConstructionScript`)